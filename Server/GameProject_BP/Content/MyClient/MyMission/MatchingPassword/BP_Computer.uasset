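; BP_Computer is a password-matching mission computer that generates and displays a random three-digit code.
; On BeginPlay it fills RandomDigits, passes them to its W_Computer widget, then starts the first BP_Answer actor in the level.
; It binds to the clear event of the BP_SoundAnalyzer tagged CorrectAnswer.
; That event's handler, despite its name CreateRandomNumbers, only makes the widget component visible.
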(event Custom|Create%20Random%20Numbers
  (Rendering|SetVisibility (Variables|Default|GetWidget) true false))

(event EventBeginPlay
  (Utilities|Array|Clear (Variables|Default|GetRandomDigits))
  (for _index (range 0 2)
    (Utilities|Array|Add (Variables|Default|GetRandomDigits) (Math|Random|RandomIntegerinRange 0 9)))
  (bind _asw_computer (Utilities|Casting|CastToW_Computer (UserInterface|GetUserWidgetObject (Variables|Default|GetWidget))))
  (Default|SetNumbers _asw_computer (Variables|Default|GetRandomDigits))
  (bind _outactors (Actor|GetAllActorsOfClass "/Game/MyClient/MyMission/MatchingPassword/BP_Answer.BP_Answer_C"))
  (bind _asbp_answer (Utilities|Casting|CastToBP_Answer (Utilities|Array|Get(acopy) _outactors)))
  (Default|Start _asbp_answer)
  (bind _outactors_2 (Actor|GetAllActorsOfClasswithTag "/Game/MyClient/MyFFT/BP_SoundAnalyzer.BP_SoundAnalyzer_C" "CorrectAnswer"))
  (bind _asbp_sound_analyzer (Utilities|Casting|CastToBP_SoundAnalyzer (Utilities|Array|Get(acopy) _outactors_2)))
  (EventDispatchers|BindEventtoSoundAnalyzerClear _asbp_sound_analyzer (delegate Custom|Create%20Random%20Numbers)))

(fn ConstructionScript)