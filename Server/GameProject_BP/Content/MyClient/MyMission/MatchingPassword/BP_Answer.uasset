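; BP_Answer is the answer keypad station of the password-matching mission.
; Start builds CorrectAnswer from the RandomDigits of BP_Computer actors in Generation order and listens for the tagged BP_SoundAnalyzer to clear.
; Box overlap enables input, letting Interact toggle W_AnswerKeypad and UI input mode once the analyzer is clear, while printing the answer on screen.
; Tab force-completes the mission without checking the answer, firing OnCompleted and showing the completion widget.
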(event OnComponentBeginOverlap(Box)
  (params (OverlappedComponent :type Primitive%20Component%20Object%20Reference) (OtherActor :type Actor%20Object%20Reference) (OtherComp :type Primitive%20Component%20Object%20Reference) (OtherBodyIndex :type Integer) (bFromSweep :type Boolean) (SweepResult :type Hit%20Result%20Structure%20%28by%20ref%29))
  (Utilities|Casting|CastToBP_Adventurer OtherActor)
  (if (Variables|Default|GetIs%20This%20Mission%20Complete?)
    (Rendering|SetVisibility (Variables|Default|GetWidget) true false)
    (else
      (Input|EnableInput (Game|GetPlayerController 0)))))

(event OnComponentEndOverlap(Box)
  (params (OverlappedComponent :type Primitive%20Component%20Object%20Reference) (OtherActor :type Actor%20Object%20Reference) (OtherComp :type Primitive%20Component%20Object%20Reference) (OtherBodyIndex :type Integer))
  (if (Variables|Default|GetIs%20This%20Mission%20Complete?)
    (Rendering|SetVisibility (Variables|Default|GetWidget) false false))
  (Input|DisableInput (Game|GetPlayerController 0)))

(event Custom|Start
  (bind _correct_answer (Variables|Default|GetCorrect%20Answer))
  (bind _outactors (Actor|GetAllActorsOfClass "/Game/MyClient/MyMission/MatchingPassword/BP_Computer.BP_Computer_C"))
  (for _array_element _outactors
    (bind _asbp_computer (Utilities|Casting|CastToBP_Computer _array_element))
    (switch int (Variables|/Game/MyClient/MyMission/MatchingPassword/BP_Computer.BP_Computer_C|GetGeneration _asbp_computer)
      (:0
        (Variables|Default|SetTemp0 (Variables|/Game/MyClient/MyMission/MatchingPassword/BP_Computer.BP_Computer_C|GetRandomDigits _asbp_computer)))
      (:1
        (Variables|Default|SetTemp1 (Variables|/Game/MyClient/MyMission/MatchingPassword/BP_Computer.BP_Computer_C|GetRandomDigits _asbp_computer)))
      (:2
        (Variables|Default|SetTemp2 (Variables|/Game/MyClient/MyMission/MatchingPassword/BP_Computer.BP_Computer_C|GetRandomDigits _asbp_computer)))))
  (Utilities|Array|Clear _correct_answer)
  (Utilities|Array|AppendArray _correct_answer (Variables|Default|GetTemp0))
  (Utilities|Array|AppendArray _correct_answer (Variables|Default|GetTemp1))
  (Utilities|Array|AppendArray _correct_answer (Variables|Default|GetTemp2))
  (bind _outactors_2 (Actor|GetAllActorsOfClasswithTag "/Game/MyClient/MyFFT/BP_SoundAnalyzer.BP_SoundAnalyzer_C" "CorrectAnswer"))
  (bind _asbp_sound_analyzer (Utilities|Casting|CastToBP_SoundAnalyzer (Utilities|Array|Get(acopy) _outactors_2)))
  (EventDispatchers|BindEventtoSoundAnalyzerClear _asbp_sound_analyzer (delegate Custom|Analyzer%20clear)))

(event Custom|Analyzer%20clear
  (Variables|Default|SetIs%20Sound%20Analyzer%20Clear? true))

(event EventBeginPlay)

(event Input|ActionEvents|InputActionInteract
  (params (Key :type Key%20Structure))
  (bind _returnvalue (Game|GetPlayerController 0))
  (bind _returnvalue_2 (Game|GetPlayerController 0))
  (:Pressed
    (if (Variables|Default|GetIs%20Sound%20Analyzer%20Clear?)
      (Development|PrintString (Utilities|String|ToString(Integer) (Utilities|Array|Length (Variables|Default|GetCorrect%20Answer))) true true "(R=1.000000,G=0.000000,B=0.847106,A=1.000000)" 6e+01)
      (for _array_element (Variables|Default|GetCorrect%20Answer)
        (Development|PrintString (Utilities|String|ToString(Integer) _array_element) true true "(R=0.000000,G=0.660000,B=1.000000,A=1.000000)" 6e+01))
      (if (Variables|Default|GetIsWidgetOpen?)
        (Widget|RemovefromParent (Variables|Default|GetKeypad%20Widget))
        (Variables|Default|SetIsWidgetOpen? false)
        (Input|SetInputModeGameOnly _returnvalue true)
        (Input|SetIgnoreMoveInput _returnvalue false)
        (Input|SetIgnoreLookInput _returnvalue false)
        (Variables|/Script/Engine.PlayerController|SetbShowMouseCursor _returnvalue false)
        (else
          (bind _returnvalue_3 (UserInterface|CreateWidget "/Game/MyClient/MyMission/MatchingPassword/W_AnswerKeypad.W_AnswerKeypad_C"))
          (bind _output_get (Variables|Default|SetKeypad%20Widget _returnvalue_3))
          (UserInterface|Viewport|AddtoViewport _output_get 0)
          (if (Variables|Default|GetIs%20This%20Mission%20Complete?)
            (bind _asw_answer_keypad (Utilities|Casting|CastToW_AnswerKeypad (Variables|Default|GetKeypad%20Widget)))
            (Default|Clear! _asw_answer_keypad)
            (Default|CallOnCompleted))
          (Variables|Default|SetIsWidgetOpen? true)
          (Input|SetIgnoreMoveInput _returnvalue_2 true)
          (Input|SetIgnoreLookInput _returnvalue_2 true)
          (Variables|/Script/Engine.PlayerController|SetbShowMouseCursor _returnvalue_2 true)
          (Input|SetInputModeGameandUI _returnvalue_2 (Variables|Default|GetKeypad%20Widget) "LockAlways" true false))))))

(event Input|KeyboardEvents|Tab
  (params (Key :type Key%20Structure))
  (:Pressed
    (if (not (Variables|Default|GetNot%20Completed?))
      (Variables|Default|SetNot%20Completed? true)
      (Default|CallOnCompleted)
      (Variables|Default|SetIs%20This%20Mission%20Complete? true)
      (Rendering|SetVisibility (Variables|Default|GetWidget) true false)
      (bind _asw_answer_keypad (Utilities|Casting|CastToW_AnswerKeypad (Variables|Default|GetKeypad%20Widget)))
      (Default|Clear! _asw_answer_keypad))))

(fn ConstructionScript)