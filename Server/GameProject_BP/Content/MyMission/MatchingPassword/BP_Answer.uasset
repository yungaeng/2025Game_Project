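; BP_Answer is the answer terminal of a password-matching mission, where the player opens a keypad.
; On BeginPlay it sorts BP_Computer actors by Generation with a small swap loop, appending all their RandomDigits to CorrectAnswer after each swap.
; A box overlap by the local adventurer enables interact input, or shows a widget once the mission is complete.
; Interact toggles W_AnswerKeypad, switching input mode, cursor and move/look locks.
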(event OnComponentBeginOverlap(Box)
  (params (OverlappedComponent :type Primitive%20Component%20Object%20Reference) (OtherActor :type Actor%20Object%20Reference) (OtherComp :type Primitive%20Component%20Object%20Reference) (OtherBodyIndex :type Integer) (bFromSweep :type Boolean) (SweepResult :type Hit%20Result%20Structure%20%28by%20ref%29))
  (bind _returnvalue (Game|GetPlayerController 0))
  (bind _asbp_adventurer (Utilities|Casting|CastToBP_Adventurer OtherActor))
  (if (Pawn|IsLocalController (Pawn|GetController _asbp_adventurer))
    (if (Variables|Default|GetIs%20This%20Mission%20Complete?)
      (Rendering|SetVisibility (Variables|Default|GetWidget) true false)
      (Input|DisableInput _returnvalue)
      (else
        (Input|EnableInput _returnvalue)))))

(event OnComponentEndOverlap(Box)
  (params (OverlappedComponent :type Primitive%20Component%20Object%20Reference) (OtherActor :type Actor%20Object%20Reference) (OtherComp :type Primitive%20Component%20Object%20Reference) (OtherBodyIndex :type Integer))
  (if (Variables|Default|GetIs%20This%20Mission%20Complete?)
    (Rendering|SetVisibility (Variables|Default|GetWidget) false false)
    (else
      (Input|DisableInput (Game|GetPlayerController 0)))))

(event EventBeginPlay
  (bind _outactors (Actor|GetAllActorsOfClass "/Game/MyMission/MatchingPassword/BP_Computer.BP_Computer_C"))
  ;[1 1 1] 버블 정렬
  (Variables|Default|SetComputer%20List _outactors)
  (for _index (range 0 1)
    (Variables|Default|Settemp (Utilities|Array|Get(acopy) (Variables|Default|GetComputer%20List) _index))
    (for _index_2 (range 1 2)
      (if (> (Variables|/Game/MyMission/MatchingPassword/BP_Computer.BP_Computer_C|GetGeneration (Utilities|Array|Get(acopy) (Variables|Default|GetComputer%20List) _index)) (Variables|/Game/MyMission/MatchingPassword/BP_Computer.BP_Computer_C|GetGeneration (Utilities|Array|Get(acopy) (Variables|Default|GetComputer%20List) _index_2)))
        (Utilities|Array|SetArrayElem (Variables|Default|GetComputer%20List) _index (Utilities|Array|Get(acopy) (Variables|Default|GetComputer%20List) _index_2))
        (Utilities|Array|SetArrayElem (Variables|Default|GetComputer%20List) _index_2 (Variables|Default|Gettemp))
        (for _array_element (Variables|Default|GetComputer%20List)
          (for _array_element_2 (Variables|/Game/MyMission/MatchingPassword/BP_Computer.BP_Computer_C|GetRandomDigits _array_element)
            (Utilities|Array|Add (Variables|Default|GetCorrect%20Answer) _array_element_2)))))))

(event Input|ActionEvents|InputActionInteract
  (params (Key :type Key%20Structure :default "None"))
  (bind _returnvalue (Game|GetPlayerController 0))
  (bind _returnvalue_2 (Game|GetPlayerController 0))
  (:Pressed
    (if (Variables|Default|GetIsWidgetOpen?)
      (Widget|RemovefromParent (Variables|Default|GetKeypad%20Widget))
      (Variables|Default|SetIsWidgetOpen? false)
      (Input|SetInputModeGameOnly _returnvalue true)
      (Input|SetIgnoreMoveInput _returnvalue false)
      (Input|SetIgnoreLookInput _returnvalue false)
      (Variables|/Script/Engine.PlayerController|SetbShowMouseCursor _returnvalue false)
      (else
        (bind _returnvalue_3 (UserInterface|CreateWidget "/Game/MyMission/MatchingPassword/W_AnswerKeypad.W_AnswerKeypad_C"))
        (bind _output_get (Variables|Default|SetKeypad%20Widget _returnvalue_3))
        (UserInterface|Viewport|AddtoViewport _output_get 0)
        (if (Variables|Default|GetIs%20This%20Mission%20Complete?)
          (bind _asw_answer_keypad (Utilities|Casting|CastToW_AnswerKeypad (Variables|Default|GetKeypad%20Widget)))
          (Default|Clear! _asw_answer_keypad))
        (Variables|Default|SetIsWidgetOpen? true)
        (Input|SetIgnoreMoveInput _returnvalue_2 true)
        (Input|SetIgnoreLookInput _returnvalue_2 true)
        (Variables|/Script/Engine.PlayerController|SetbShowMouseCursor _returnvalue_2 true)
        (Input|SetInputModeGameandUI _returnvalue_2 (Variables|Default|GetKeypad%20Widget) "LockAlways" true false)))))

(fn ConstructionScript)