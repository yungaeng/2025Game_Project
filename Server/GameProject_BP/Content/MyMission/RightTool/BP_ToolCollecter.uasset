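; Tool collector station for a fix mission, showing a progress or completion widget while the local player's BP_Adventurer overlaps its box.
; UpdateCollectercount increments the tool widget's count up to its maximum, flags completion, and reports the mission ID to MyGameInstance via SetMission.
; Tick polls game data into CollectedToolsInCollecter, with the ID selecting the armory or control fix mission value.
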(event OnComponentBeginOverlap(Box)
  (params (OverlappedComponent :type Primitive%20Component%20Object%20Reference) (OtherActor :type Actor%20Object%20Reference) (OtherComp :type Primitive%20Component%20Object%20Reference) (OtherBodyIndex :type Integer) (bFromSweep :type Boolean) (SweepResult :type Hit%20Result%20Structure%20%28by%20ref%29))
  (bind _asbp_adventurer (Utilities|Casting|CastToBP_Adventurer OtherActor))
  (if (Pawn|IsLocalController (Pawn|GetController _asbp_adventurer))
    (if (Variables|Default|GetIs%20This%20Mission%20Complete?)
      (Rendering|SetVisibility (Variables|Default|GetCompleteWidget) true false)
      (Variables|Default|SetIs%20on%20Collecter? true)
      (else
        (Rendering|SetVisibility (Variables|Default|GetToolWidget) true false)))))

(event OnComponentEndOverlap(Box)
  (params (OverlappedComponent :type Primitive%20Component%20Object%20Reference) (OtherActor :type Actor%20Object%20Reference) (OtherComp :type Primitive%20Component%20Object%20Reference) (OtherBodyIndex :type Integer))
  (Utilities|Casting|CastToBP_Adventurer OtherActor)
  (if (Variables|Default|GetIs%20This%20Mission%20Complete?)
    (Rendering|SetVisibility (Variables|Default|GetCompleteWidget) false false))
  (Rendering|SetVisibility (Variables|Default|GetToolWidget) false false)
  (Variables|Default|SetIs%20on%20Collecter? false))

(event Custom|Update%20Collecter%20count
  (bind _asw_collect_tools (Utilities|Casting|CastToW_CollectTools (UserInterface|GetUserWidgetObject (Variables|Default|GetToolWidget))))
  (if (> (Variables|/Game/MyMission/RightTool/W_CollectTools.W_CollectTools_C|GetMax%20Tools _asw_collect_tools) (Variables|/Game/MyMission/RightTool/W_CollectTools.W_CollectTools_C|GetCollected%20Tools _asw_collect_tools))
    (bind _output_get (Variables|/Game/MyMission/RightTool/W_CollectTools.W_CollectTools_C|SetCollected%20Tools _asw_collect_tools (+ (Variables|/Game/MyMission/RightTool/W_CollectTools.W_CollectTools_C|GetCollected%20Tools _asw_collect_tools) 1)))
    (Variables|Default|SetCollected%20Tools%20in%20collecter _output_get)
    (if (== (Variables|/Game/MyMission/RightTool/W_CollectTools.W_CollectTools_C|GetMax%20Tools _asw_collect_tools) (Variables|/Game/MyMission/RightTool/W_CollectTools.W_CollectTools_C|GetCollected%20Tools _asw_collect_tools))
      (Variables|Default|SetIs%20This%20Mission%20Complete? true))
    (CallFunction|Send)))

(event EventTick
  (params (DeltaSeconds :type Float%20%28single-precision%29))
  (bind _returnvalue (CallFunction|Recv (Variables|Default|GetID)))
  (Variables|Default|SetCollected%20Tools%20in%20collecter _returnvalue))

(fn ConstructionScript)

(fn Send
  (bind _asmy_game_instance (Utilities|Casting|CastToMyGameInstance (Game|GetGameInstance)))
  (Class|MyGameInstance|SetMission _asmy_game_instance (Variables|Default|GetID)))

(fn Recv
  (params (NewParam :type Integer))
  (bind _returnvalue (Game|GetGameInstance))
  (if (Math|Conversions|ToBoolean(Integer) (+ NewParam -1))
    (bind _asmy_game_instance (Utilities|Casting|CastToMyGameInstance _returnvalue))
    (bind _returnvalue_2 (Class|MyGameInstance|GetGameData _asmy_game_instance))
    (return (.armory_fix_mission _returnvalue_2))
    (else
      (bind _asmy_game_instance_2 (Utilities|Casting|CastToMyGameInstance _returnvalue))
      (bind _returnvalue_3 (Class|MyGameInstance|GetGameData _asmy_game_instance_2))
      (return (.control_fix_mission _returnvalue_3)))))