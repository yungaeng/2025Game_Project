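; Microphone "screaming" mission actor, enabled once the tagged BP_SoundAnalyzer is cleared.
; While BP_Adventurer is in its box, AudioCapture converts the mic envelope into a loudness value shown on W_ScreemingWidget.
; Loud input spawns A_EchoGenerate through a timer-reset gate, and over three cumulative seconds of it completes the mission and swaps to the completion widget.
; Pressing Tab inside the box completes it immediately.
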(event OnAudioEnvelopeValue(AudioCapture)
  (params (EnvelopeValue :type Float%20%28single-precision%29))
  (bind _output_get (Variables|Default|SetHow%20Loud (* (* (/ (Math|Float|Clamp(Float) EnvelopeValue 0.0 0.5) 0.5) 2.2) 1e+02)))
  (bind _asw_screeming_widget (Utilities|Casting|CastToW_ScreemingWidget (UserInterface|GetUserWidgetObject (Variables|Default|GetWidget))))
  (if (Variables|Default|GetIs%20This%20Mission%20Complete?)
    (Variables|Default|SetHow%20Loud 1e+02))
  (Variables|/Game/Client/MyMission/TogetherScreeming/W_ScreemingWidget.W_ScreemingWidget_C|SetHow%20Loud%20in%20widget _asw_screeming_widget _output_get))

(event OnComponentBeginOverlap(Box)
  (params (OverlappedComponent :type Primitive%20Component%20Object%20Reference) (OtherActor :type Actor%20Object%20Reference) (OtherComp :type Primitive%20Component%20Object%20Reference) (OtherBodyIndex :type Integer) (bFromSweep :type Boolean) (SweepResult :type Hit%20Result%20Structure%20%28by%20ref%29))
  (Utilities|Casting|CastToBP_Adventurer OtherActor)
  (Input|EnableInput (Game|GetPlayerController 0))
  (if (Variables|Default|GetIs%20Start?)
    (if (Variables|Default|GetIs%20This%20Mission%20Complete?)
      (Rendering|SetVisibility (Variables|Default|GetComplete%20Widget) true false)
      (else
        (Components|Activation|Activate (Variables|Default|GetAudioCapture) false)
        (Rendering|SetVisibility (Variables|Default|GetWidget) true false)))))

(event OnComponentEndOverlap(Box)
  (params (OverlappedComponent :type Primitive%20Component%20Object%20Reference) (OtherActor :type Actor%20Object%20Reference) (OtherComp :type Primitive%20Component%20Object%20Reference) (OtherBodyIndex :type Integer))
  (Utilities|Casting|CastToBP_Adventurer OtherActor)
  (Input|DisableInput (Game|GetPlayerController 0))
  (if (Variables|Default|GetIs%20Start?)
    (if (Variables|Default|GetIs%20This%20Mission%20Complete?)
      (Rendering|SetVisibility (Variables|Default|GetComplete%20Widget) false false))
    (Components|Activation|Deactivate (Variables|Default|GetAudioCapture))
    (Rendering|SetVisibility (Variables|Default|GetWidget) false false)))

(event Custom|Start
  (Variables|Default|SetIs%20Start? true))

(event Custom|ResetSpawnGate
  (Utilities|FlowControl|Gate false) ; enters at Open
)

(event EventTick
  (params (DeltaSeconds :type Float%20%28single-precision%29))
  (if (Variables|Default|GetIs%20Start?)
    (if (>= (Variables|Default|GetHow%20Loud) 95.0)
      (if (not (Variables|Default|GetIs%20This%20Mission%20Complete?))
        (Utilities|FlowControl|Sequence
          (:then_0
            (Utilities|FlowControl|Gate false :!label _label
              (:Exit
                (bind _returnvalue (Actor|GetActorOfClass "/Game/Client/MyImposter/BP_Imposter.BP_Imposter_C"))
                (bind _asbp_imposter (Utilities|Casting|CastToBP_Imposter _returnvalue))
                (Game|SpawnActorfromClass "/Game/Client/MyEcholation/A_EchoGenerate.A_EchoGenerate_C" (Math|Transform|MakeTransform (Transformation|GetActorLocation) "0, 0, 0" "1.000000,1.000000,1.000000") "Undefined" "MultiplyWithRoot" 0 "(R=1.000000,G=1.000000,B=1.000000,A=1.000000)" 5e+02 0.0 (Variables|/Game/Client/MyImposter/BP_Imposter.BP_Imposter_C|GetCameraImposter _asbp_imposter) 0)
                (Utilities|FlowControl|Sequence
                  (:then_0
                    (goto _label Close))
                  (:then_1
                    (Utilities|Time|SetTimerbyEvent (delegate Custom|ResetSpawnGate) 0.5))))))
          (:then_1
            (bind _output_get (Variables|Default|SetMax%20Time (+ (Variables|Default|GetMax%20Time) DeltaSeconds)))
            (if (> _output_get 3.0)
              (Variables|Default|SetIs%20This%20Mission%20Complete? true)
              (Default|CallOnCompleted)
              (if (Variables|Default|Getfirst%20Clear?)
                (Rendering|SetVisibility (Variables|Default|GetWidget) false false)
                (Rendering|SetVisibility (Variables|Default|GetComplete%20Widget) true false)
                (Components|Activation|Deactivate (Variables|Default|GetAudioCapture))
                (Variables|Default|Setfirst%20Clear? false)))))))))

(event EventBeginPlay
  (bind _outactors (Actor|GetAllActorsOfClasswithTag "/Game/Client/MyFFT/BP_SoundAnalyzer.BP_SoundAnalyzer_C" "Screeming"))
  (bind _asbp_sound_analyzer (Utilities|Casting|CastToBP_SoundAnalyzer (Utilities|Array|Get(acopy) _outactors)))
  (EventDispatchers|BindEventtoSoundAnalyzerClear _asbp_sound_analyzer (delegate Custom|Start)))

(event Input|KeyboardEvents|Tab
  (params (Key :type Key%20Structure))
  (:Pressed
    (if (not (Variables|Default|GetNot%20Completed?))
      (Variables|Default|SetNot%20Completed? true)
      (Variables|Default|SetIs%20This%20Mission%20Complete? true)
      (Default|CallOnCompleted)
      (Rendering|SetVisibility (Variables|Default|GetComplete%20Widget) true false)
      (Components|Activation|Deactivate (Variables|Default|GetAudioCapture))
      (Rendering|SetVisibility (Variables|Default|GetWidget) false false)
      (Variables|Default|Setfirst%20Clear? false))))

(fn ConstructionScript)