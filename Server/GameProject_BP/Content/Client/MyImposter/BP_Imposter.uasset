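; BP_Imposter is the playable Imposter character, which attacks Adventurers with a melee weapon and emits echoes from its actions.
; Right mouse plays a Smash montage, locked by a DoOnce until it completes.
; Any weapon overlap spawns an A_EchoGenerate linked to the Imposter camera, then damages Adventurers with a slap sound.
; Foot notifies spawn wider-range echoes, Tick stores ground speed, and jump is unwired.
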(event OnComponentBeginOverlap(ImposterWeapon)
  (params (OverlappedComponent :type Primitive%20Component%20Object%20Reference) (OtherActor :type Actor%20Object%20Reference) (OtherComp :type Primitive%20Component%20Object%20Reference) (OtherBodyIndex :type Integer) (bFromSweep :type Boolean) (SweepResult :type Hit%20Result%20Structure%20%28by%20ref%29))
  (Game|SpawnActorfromClass "/Game/Client/MyEcholation/A_EchoGenerate.A_EchoGenerate_C" (Math|Transform|MakeTransform (Transformation|GetActorLocation) "0, 0, 0" "1.000000,1.000000,1.000000") "Undefined" "MultiplyWithRoot" 0 "(R=1.000000,G=1.000000,B=1.000000,A=1.000000)" 5e+02 0.0 (Variables|Default|GetCameraImposter) 0)
  (bind _asbp_adventurer (Utilities|Casting|CastToBP_Adventurer OtherActor))
  (Default|TakeDamage _asbp_adventurer)
  (Audio|PlaySound2D "/Game/Client/MyImposter/hard-slap.hard-slap" 0.2 1.0 0.0 0 0))

(event Custom|CE_FootNotify
  (Game|SpawnActorfromClass "/Game/Client/MyEcholation/A_EchoGenerate.A_EchoGenerate_C" (Math|Transform|MakeTransform (Transformation|GetActorLocation) "0, 0, 0" "1.000000,1.000000,1.000000") "Undefined" "MultiplyWithRoot" 0 "(R=1.000000,G=1.000000,B=1.000000,A=1.000000)" 1e+03 0.0 (Variables|Default|GetCameraImposter) 0))

(event Input|EnhancedActionEvents|EnhancedInputActionIA_Jump_I
  (params (ActionValue :type Boolean) (ElapsedSeconds :type Float%20%28double-precision%29) (TriggeredSeconds :type Float%20%28double-precision%29) (InputAction :type Input%20Action%20Object%20Reference :default "/Game/Client/MyImposter/IA_Jump_I.IA_Jump_I")))

(event EventBeginPlay)

(event Collision|EventActorBeginOverlap
  (params (OtherActor :type Actor%20Object%20Reference)))

(event EventTick
  (params (DeltaSeconds :type Float%20%28single-precision%29))
  ;[1 1 1] 캐릭터의 속도를 저장한다.
  (Variables|Default|SetGround%20Speed (Math|Vector|VectorLengthXY (Variables|/Script/Engine.MovementComponent|GetVelocity (Variables|Character|GetCharacterMovement)))))

(event Input|MouseEvents|RightMouseButton
  (params (Key :type Key%20Structure))
  (:Pressed
    (Utilities|FlowControl|DoOnce false :!label _label
      (:Completed
        (Animation|Montage|PlayMontage (Variables|Character|GetMesh) "/Game/Client/MyImposter/ImposterAnimation/ImposterAnimMontage.ImposterAnimMontage" 1.5 0.0 "Smash"
          (:OnCompleted
            (goto _label Reset)))))))

(fn ConstructionScript)