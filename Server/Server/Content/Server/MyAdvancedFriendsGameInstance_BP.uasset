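; Game instance that drives menu navigation, multiplayer sessions, character spawning and the game-over check.
; Show events clear widgets and display cached menus, except the mission widget, which overlays without clearing.
; Session creation opens the lobby as listen server; accepted invites rejoin as a non-imposter adventurer.
; GameOverCheck updates the mission checklist and travels to NewWorld on game over, full mission completion or negative adventurer TotalHit.
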(event Custom|Create%20Session
  ;[1 1 1] 세션 만들기
  (Viewport|RemoveAllWidgets)
  (|AdvancedSession 0 (Game|GetPlayerController 0) 100 0 false true false true true false false false true false true
    (:OnSuccess
      (Game|OpenLevel(byObjectReference) "/Game/MyMap/lobby.lobby" true "listen")
      (CallFunction|ShowLobby)
      (Class|MyAdvancedFriendsGameInstance|SendRoom))))

(event Custom|show%20connect
  ;[1 1 1] connect
  (Viewport|RemoveAllWidgets)
  (if (Utilities|IsValid (Variables|Default|Getconnect))
    _
    (else
      (bind _returnvalue (UserInterface|CreateWidget "/Game/Server/MainMenu/connect.connect_C" (Game|GetPlayerController 0)))
      (bind _output_get (Variables|Default|Setconnect _returnvalue))))
  (UserInterface|Viewport|AddtoViewport _output_get 0))

(event Custom|show%20host
  ;[1 1 1] hostmenu
  (Viewport|RemoveAllWidgets)
  (if (Utilities|IsValid (Variables|Default|Gethost))
    _
    (else
      (bind _returnvalue (UserInterface|CreateWidget "/Game/Server/MainMenu/HostMenu.HostMenu_C" (Game|GetPlayerController 0)))
      (bind _output_get (Variables|Default|Sethost _returnvalue))))
  (UserInterface|Viewport|AddtoViewport _output_get 0))

(event Custom|show%20mission%20widget
  ;[1 1 1] 미션 완료 위젯 보이기
  (if (Utilities|IsValid (Variables|Default|Getmission))
    _
    (else
      (bind _returnvalue (UserInterface|CreateWidget "/Game/MyMission/CheckMissionComplete.CheckMissionComplete_C"))
      (bind _output_get (Variables|Default|Setmission _returnvalue))))
  (UserInterface|Viewport|AddtoViewport _output_get 0))

(event Custom|show%20lobby
  ;[1 1 1] lobby
  (Viewport|RemoveAllWidgets)
  (if (Utilities|IsValid (Variables|Default|Getlobby))
    _
    (else
      (bind _returnvalue (UserInterface|CreateWidget "/Game/Server/Lobby/W_LobbyUI.W_LobbyUI_C" (Game|GetPlayerController 0)))
      (bind _output_get (Variables|Default|Setlobby _returnvalue))))
  (UserInterface|Viewport|AddtoViewport _output_get 0))

(event Custom|show%20join
  ;[1 1 1] join menu
  (Viewport|RemoveAllWidgets)
  (if (Utilities|IsValid (Variables|Default|Getjoin))
    _
    (else
      (bind _returnvalue (UserInterface|CreateWidget "/Game/Server/MainMenu/ServerMenu.ServerMenu_C" (Game|GetPlayerController 0)))
      (bind _output_get (Variables|Default|Setjoin _returnvalue))))
  (UserInterface|Viewport|AddtoViewport _output_get 0))

(event Custom|show%20mainmenu
  ;[1 1 1] mainmenu
  (Viewport|RemoveAllWidgets)
  (if (Utilities|IsValid (Variables|Default|Getmain))
    _
    (else
      (bind _returnvalue (UserInterface|CreateWidget "/Game/Server/MainMenu/MainMenu.MainMenu_C" (Game|GetPlayerController 0)))
      (bind _output_get (Variables|Default|Setmain _returnvalue))))
  (UserInterface|Viewport|AddtoViewport _output_get 0))

(event EventOnSessionInviteAccepted
  (params (LocalPlayerNum :type Integer) (PersonInvited :type BP%20Unique%20Net%20Id%20Structure) (SessionToJoin :type Blueprint%20Session%20Result%20Structure%20%28by%20ref%29))
  (bind _returnvalue (Game|GetPlayerController 0))
  ;[1 1 1] 초대 수락
  (Viewport|RemoveAllWidgets)
  (|DestroySession _returnvalue
    (:OnSuccess
      (Variables|Default|Setchar "/Game/MyAdventurer/BP_Adventurer.BP_Adventurer_C")
      (Variables|Default|Setis%20imposter false)
      (|JoinSession _returnvalue SessionToJoin))))

(fn GameOverCheck
  (params (tool1 :type BP%20Tool%20Collecter%20Object%20Reference) (tool2 :type BP%20Tool%20Collecter%20Object%20Reference) (scream :type BP%20Screeming%20Object%20Reference) (answer :type BP%20Answer%20Object%20Reference) (note :type BP%20Random%20Note%20Player%20Object%20Reference) (temp :type BP%20Fix%20Temperature%20Object%20Reference) (adventrue :type BP%20Adventurer%20Object%20Reference) (widget :type Check%20Mission%20Complete%20Object%20Reference))
  (bind _is_this_mission_complete_ (Variables|/Game/MyMission/RightTool/BP_ToolCollecter.BP_ToolCollecter_C|GetIs%20This%20Mission%20Complete? tool2))
  (bind _is_this_mission_complete__2 (Variables|/Game/MyMission/RightSyllable/BP_RandomNotePlayer.BP_RandomNotePlayer_C|GetIs%20This%20Mission%20Complete? note))
  (bind _is_this_mission_complete__3 (Variables|/Game/MyMission/FixTemperature/BP_FixTemperature.BP_FixTemperature_C|GetIs%20This%20Mission%20Complete? temp))
  (bind _is_this_mission_complete__4 (Variables|/Game/MyMission/TogetherScreeming/BP_Screeming.BP_Screeming_C|GetIs%20This%20Mission%20Complete? scream))
  (bind _is_this_mission_complete__5 (Variables|/Game/MyMission/MatchingPassword/BP_Answer.BP_Answer_C|GetIs%20This%20Mission%20Complete? answer))
  (bind _is_this_mission_complete__6 (Variables|/Game/MyMission/RightTool/BP_ToolCollecter.BP_ToolCollecter_C|GetIs%20This%20Mission%20Complete? tool1))
  (bind _returnvalue (Class|MyAdvancedFriendsGameInstance|GetGameOverState))
  (if _returnvalue
    (Game|OpenLevel(byName) "NewWorld" :!label _label)
    (Class|AdvancedSessionsLibrary|ServerTravel "NewWorld" false false)
    (elif (Math|Boolean|ANDBoolean _is_this_mission_complete__6 _is_this_mission_complete_ _is_this_mission_complete__4 _is_this_mission_complete__5 _is_this_mission_complete__2 _is_this_mission_complete__3)
      (goto _label)
      (else
        (CallFunction|UpdateMissionCheck _is_this_mission_complete__6 _is_this_mission_complete_ _is_this_mission_complete__4 _is_this_mission_complete__5 _is_this_mission_complete__2 _is_this_mission_complete__3 widget adventrue)
        (if (< (Variables|/Game/MyAdventurer/BP_Adventurer.BP_Adventurer_C|GetTotal%20Hit adventrue) 0)
          (Class|MyAdvancedFriendsGameInstance|SendAttack)
          (goto _label))))))

(fn SpawnCharacterandShowWidget
  (params (Loc :type Transform))
  (bind _returnvalue (Game|GetPlayerController 0))
  (Pawn|UnPossess _returnvalue)
  (bind _returnvalue_2 (Game|SpawnActorfromClass (Variables|Default|Getchar) Loc "Undefined" "MultiplyWithRoot" 0 0))
  (Pawn|Possess _returnvalue _returnvalue_2)
  (CallFunction|ShowMissionWidget))

(fn UpdateMissionCheck
  (params (tool1 :type Boolean) (too2 :type Boolean) (scream :type Boolean) (answer :type Boolean) (note :type Boolean) (temp :type Boolean) (NewParam :type Check%20Mission%20Complete%20Object%20Reference) (NewParam1 :type BP%20Adventurer%20Object%20Reference))
  (Default|Update NewParam tool1 too2 scream answer note temp (== (Variables|/Game/MyAdventurer/BP_Adventurer.BP_Adventurer_C|GetTotal%20Hit NewParam1) 3)))