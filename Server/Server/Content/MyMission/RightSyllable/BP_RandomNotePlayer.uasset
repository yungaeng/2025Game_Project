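; Note-memory puzzle TV for the RightSyllable mission, activated when the tagged BP_SoundAnalyzer is cleared.
; Interact inside its box plays three random notes with material wave pulses and enables BP_SetNote collision.
; AddNoteIndex collects the player's notes, compares the sequence, then disables note collision; correct answers update the progress widget.
; The third success completes the mission, and Tab forces completion.
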(event OnComponentBeginOverlap(Box)
  (params (OverlappedComponent :type Primitive%20Component%20Object%20Reference) (OtherActor :type Actor%20Object%20Reference) (OtherComp :type Primitive%20Component%20Object%20Reference) (OtherBodyIndex :type Integer) (bFromSweep :type Boolean) (SweepResult :type Hit%20Result%20Structure%20%28by%20ref%29))
  (Utilities|Casting|CastToBP_Adventurer OtherActor)
  (if (Variables|Default|GetIs%20This%20Mission%20Complete?)
    (Rendering|SetVisibility (Variables|Default|GetComplete) true false)
    (else
      (Input|EnableInput (Game|GetPlayerController 0)))))

(event OnComponentEndOverlap(Box)
  (params (OverlappedComponent :type Primitive%20Component%20Object%20Reference) (OtherActor :type Actor%20Object%20Reference) (OtherComp :type Primitive%20Component%20Object%20Reference) (OtherBodyIndex :type Integer))
  (Utilities|Casting|CastToBP_Adventurer OtherActor)
  (Input|DisableInput (Game|GetPlayerController 0))
  (Rendering|SetVisibility (Variables|Default|GetComplete) false false))

(event Custom|Random%20Notes
  ;[1 1 1] 0~7 랜덤한 숫자 세개 뽑기
  (for _index (range 0 2)
    (Utilities|Array|Add (Variables|Default|Get%20NoteIndexArray) (Math|Random|RandomIntegerinRange 0 7))))

(event Custom|Play%20sound
  (bind _returnvalue (Transformation|GetActorLocation))
  ;[1 1 1] 랜덤한 숫자 3를 사운드 인덱스로 적용 시켜서 플레이
  (if (Variables|Default|GetIs%20Start?)
    (Utilities|FlowControl|Delay 1.2)
    (Audio|PlaySoundatLocation _returnvalue)
    (|Wave)
    (|Playsoundatlocation2 _returnvalue)
    (|Wave_2)
    (|Playsoundatloacation3 _returnvalue)
    (|Wave_3)
    (bind _returnvalue_2 (Actor|GetActorOfClass "/Game/MyMission/RightSyllable/BP_SetNote.BP_SetNote_C"))
    (Default|EnableNoteCollision _returnvalue_2)))

(event Custom|Add%20Note%20Index
  (params (NoteIndex :type Integer))
  (Utilities|Array|Add (Variables|Default|GetPlayer%20Input%20Array) NoteIndex)
  (if (== (Utilities|Array|Length (Variables|Default|Get%20NoteIndexArray)) (Utilities|Array|Length (Variables|Default|GetPlayer%20Input%20Array)))
    (CallFunction|CheckPlayerAnswer)
    (bind _outactors (Actor|GetAllActorsOfClass "/Game/MyMission/RightSyllable/BP_SetNote.BP_SetNote_C"))
    (for _array_element _outactors
      (Default|DisableNoteCollision _array_element))))

(event Custom|Start
  (Variables|Default|SetIs%20Start? true)
  ;[1 1 1] 시작하자마자 랜덤 숫자 부여
  (CallFunction|RandomNotes)
  (bind _returnvalue (Rendering|Material|CreateDynamicMaterialInstance (Variables|Default|GetPlane) 0 "/Game/MyMission/RightSyllable/MI_NotePlayerTV.MI_NotePlayerTV" "None" :!class /Script/Engine.PrimitiveComponent))
  (bind _output_get (Variables|Default|SetTV%20Material _returnvalue))
  (Rendering|Material|SetMaterial (Variables|Default|GetPlane) 0 _output_get))

(event EventBeginPlay
  (bind _outactors (Actor|GetAllActorsOfClasswithTag "/Game/MyFFT/BP_SoundAnalyzer.BP_SoundAnalyzer_C" "RightSyllable"))
  (bind _asbp_sound_analyzer (Utilities|Casting|CastToBP_SoundAnalyzer (Utilities|Array|Get(acopy) _outactors)))
  (EventDispatchers|BindEventtoSoundAnalyzerClear _asbp_sound_analyzer (delegate Custom|Start)))

(event Input|ActionEvents|InputActionInteract
  (params (Key :type Key%20Structure :default "None"))
  (:Pressed
    (if (Variables|Default|GetIs%20Start?)
      (if (Variables|Default|GetIs%20Answer%20Is%20Correct?)
        (if (not (> (Variables|Default|GetQuestion%20number) 2))
          (Utilities|Array|Clear (Variables|Default|GetPlayer%20Input%20Array))
          (Utilities|Array|Clear (Variables|Default|Get%20NoteIndexArray))
          (CallFunction|RandomNotes)
          (CallFunction|PlaySound))
        (else
          (CallFunction|PlaySound))))))

(event Input|KeyboardEvents|Tab
  (params (Key :type Key%20Structure :default "None"))
  (:Pressed
    (if (not (Variables|Default|GetNot%20Completed?))
      (Variables|Default|SetNot%20Completed? true)
      (Variables|Default|SetIs%20This%20Mission%20Complete? true)
      (Rendering|SetVisibility (Variables|Default|GetComplete) true false)
      (Variables|Default|SetQuestion%20number 3)
      (Default|CallOnCompleted))))

(fn ConstructionScript)

(fn CheckPlayerAnswer
  (bind _index (Utilities|FlowControl|ForLoopwithBreak 0 (- (Utilities|Array|Length (Variables|Default|Get%20NoteIndexArray)) 1))
    (:LoopBody
      (if (not (== (Utilities|Array|Get(acopy) (Variables|Default|Get%20NoteIndexArray) _index) (Utilities|Array|Get(acopy) (Variables|Default|GetPlayer%20Input%20Array) _index)))
        (Utilities|Array|Clear (Variables|Default|GetPlayer%20Input%20Array))
        (Variables|Default|SetIs%20Answer%20Is%20Correct? false)
        (return)))
    (:Completed
      (Variables|Default|SetIs%20Answer%20Is%20Correct? true)
      (Variables|Default|SetQuestion%20number (+ (Variables|Default|GetQuestion%20number) 1))
      (bind _asw_random_note_player_question_number (Utilities|Casting|CastToW_RandomNotePlayer_QuestionNumber (UserInterface|GetWidget (Variables|Default|GetWidget))))
      (Default|UpdateProgress _asw_random_note_player_question_number)
      (if (== (Variables|Default|GetQuestion%20number) 3)
        (Variables|Default|SetIs%20This%20Mission%20Complete? true)
        (Default|CallOnCompleted))
      (return))))