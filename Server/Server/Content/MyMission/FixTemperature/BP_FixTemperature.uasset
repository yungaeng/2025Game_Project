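; Mission actor for fixing temperature, whose dynamic material shifts over RequiredTime as HeatPercent falls.
; Top and Bottom components set the material's vertical range, and an event toggles its thermal-vision parameter.
; BP_Adventurer overlap enables input; holding Interact over three seconds, via a gated next-tick Hold macro, resets temperature, completes the mission and notifies the game instance.
; Tab also triggers a one-time reset; the HeatPercent-based failure check is disconnected.
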(event OnComponentBeginOverlap(Capsule)
  (params (OverlappedComponent :type Primitive%20Component%20Object%20Reference) (OtherActor :type Actor%20Object%20Reference) (OtherComp :type Primitive%20Component%20Object%20Reference) (OtherBodyIndex :type Integer) (bFromSweep :type Boolean) (SweepResult :type Hit%20Result%20Structure%20%28by%20ref%29))
  (Utilities|Casting|CastToBP_Adventurer OtherActor)
  (Input|EnableInput (Game|GetPlayerController 0)))

(event OnComponentEndOverlap(Capsule)
  (params (OverlappedComponent :type Primitive%20Component%20Object%20Reference) (OtherActor :type Actor%20Object%20Reference) (OtherComp :type Primitive%20Component%20Object%20Reference) (OtherBodyIndex :type Integer))
  (Input|DisableInput (Game|GetPlayerController 0)))

(event Custom|ResetTemperature
  (Variables|Default|SetHeatPercent 0.0)
  (bind _output_get (Variables|Default|SetElapsedTime 0.0))
  (Rendering|Material|SetScalarParameterValue (Variables|Default|GetDynamicMaterial) (Variables|Default|GetName_Alpha) _output_get :!class /Script/Engine.MaterialInstanceDynamic)
  (Variables|Default|SetIs%20This%20Mission%20Complete? true)
  (Default|CallOnCompleted)
  (bind _asmy_advanced_friends_game_instance (Utilities|Casting|CastToMyAdvancedFriendsGameInstance (Game|GetGameInstance)))
  (Class|MyAdvancedFriendsGameInstance|SendMission _asmy_advanced_friends_game_instance 5))

(event Custom|ToggleTempVision
  (params (bOn :type Boolean))
  (bind _dynamicmaterial (Variables|Default|GetDynamicMaterial))
  (if bOn
    (Rendering|Material|SetScalarParameterValue _dynamicmaterial "ThermalVision" 1.0 :!class /Script/Engine.MaterialInstanceDynamic)
    (else
      (Rendering|Material|SetScalarParameterValue _dynamicmaterial "ThermalVision" 0.0 :!class /Script/Engine.MaterialInstanceDynamic))))

(event EventBeginPlay
  (CallFunction|InitDynamicMaterial)
  (Variables|Default|SetElapsedTime 0.0))

(event EventTick
  (params (DeltaSeconds :type Float%20%28single-precision%29))
  (bind _output_get (Variables|Default|SetElapsedTime (+ DeltaSeconds (Variables|Default|GetElapsedTime))))
  (Rendering|Material|SetScalarParameterValue (Variables|Default|GetDynamicMaterial) (Variables|Default|GetName_Alpha) (Math|Float|Min(Float) (/ _output_get (Variables|Default|GetRequiredTime)) 1.0) :!class /Script/Engine.MaterialInstanceDynamic)
  (Variables|Default|SetHeatPercent (* (- 1.0 (/ (Variables|Default|GetElapsedTime) (Variables|Default|GetRequiredTime))) 1e+02)))

(event Input|ActionEvents|InputActionInteract
  (params (Key :type Key%20Structure :default "None"))
  (:Pressed
    (Utilities|Hold :!label _label
      (:On%20Holding%20Tick
        (bind _output_get (Variables|Default|SetHoldingTime (+ (Variables|Default|GetHoldingTime) (Utilities|Time|GetWorldDeltaSeconds))))
        (if (> _output_get 3.0)
          (if (not (Variables|Default|GetFix%20Once))
            (CallFunction|ResetTemperature)
            (Variables|Default|SetFix%20Once true))))
      (:Complete
        (Variables|Default|SetHoldingTime 0.0))))
  (:Released
    (goto _label Leave)))

(event Input|KeyboardEvents|Tab
  (params (Key :type Key%20Structure :default "None"))
  (:Pressed
    (if (not (Variables|Default|GetNot%20Completed?))
      (Variables|Default|SetNot%20Completed? true)
      (CallFunction|ResetTemperature))))

(fn ConstructionScript)

(fn ToggleThermalVision
  (params (bOn :type Boolean))
  (if bOn
    _))

(fn InitDynamicMaterial
  (bind _bottom (Variables|Default|GetBottom))
  (bind _returnvalue (Transformation|GetWorldLocation _bottom))
  (bind _returnvalue_2 (Rendering|Material|CreateDynamicMaterialInstance (Variables|Default|GetStaticMesh) 0 "/Game/MyMission/FixTemperature/M_FixTemperature.M_FixTemperature" "None" :!class /Script/Engine.PrimitiveComponent))
  (bind _output_get (Variables|Default|SetDynamicMaterial _returnvalue_2))
  (Rendering|Material|SetScalarParameterValue _output_get (Variables|Default|GetName_Alpha) 0.0 :!class /Script/Engine.MaterialInstanceDynamic)
  (Rendering|Material|SetMaterial (Variables|Default|GetStaticMesh) 0 (Variables|Default|GetDynamicMaterial))
  (Rendering|Material|SetScalarParameterValue (Variables|Default|GetDynamicMaterial) "BottomPosition" (.z _returnvalue) :!class /Script/Engine.MaterialInstanceDynamic)
  (Rendering|Material|SetScalarParameterValue (Variables|Default|GetDynamicMaterial) "Height" (- (.z (Transformation|GetWorldLocation (Variables|Default|GetTop))) (.z _returnvalue)) :!class /Script/Engine.MaterialInstanceDynamic)
  (return true))