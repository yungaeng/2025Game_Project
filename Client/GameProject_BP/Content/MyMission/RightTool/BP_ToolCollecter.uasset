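; BP_ToolCollecter is a mission drop-off point that tracks collected tools and signals when the collection is complete.
; Its box overlap shows the adventurer either the tool-count widget or the completion widget, enabling input while incomplete.
; UpdateCollectercount increments the count stored in W_CollectTools and fires the completion call at the maximum.
; While input is enabled, Tab acts as a one-time shortcut that force-completes the mission with a hardcoded count.
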(event OnComponentBeginOverlap(Box)
  (params (OverlappedComponent :type Primitive%20Component%20Object%20Reference) (OtherActor :type Actor%20Object%20Reference) (OtherComp :type Primitive%20Component%20Object%20Reference) (OtherBodyIndex :type Integer) (bFromSweep :type Boolean) (SweepResult :type Hit%20Result%20Structure%20%28by%20ref%29))
  (Utilities|Casting|CastToBP_Adventurer OtherActor)
  (if (Variables|Default|GetIs%20This%20Mission%20Complete?)
    (Rendering|SetVisibility (Variables|Default|GetCompleteWidget) true false)
    (Variables|Default|SetIs%20on%20Collecter? true)
    (else
      (Input|EnableInput (Game|GetPlayerController 0))
      (Rendering|SetVisibility (Variables|Default|GetToolWidget) true false))))

(event OnComponentEndOverlap(Box)
  (params (OverlappedComponent :type Primitive%20Component%20Object%20Reference) (OtherActor :type Actor%20Object%20Reference) (OtherComp :type Primitive%20Component%20Object%20Reference) (OtherBodyIndex :type Integer))
  (Utilities|Casting|CastToBP_Adventurer OtherActor)
  (Input|DisableInput (Game|GetPlayerController 0))
  (if (Variables|Default|GetIs%20This%20Mission%20Complete?)
    (Rendering|SetVisibility (Variables|Default|GetCompleteWidget) false false))
  (Rendering|SetVisibility (Variables|Default|GetToolWidget) false false)
  (Variables|Default|SetIs%20on%20Collecter? false))

(event Custom|Update%20Collecter%20count
  (bind _asw_collect_tools (Utilities|Casting|CastToW_CollectTools (UserInterface|GetUserWidgetObject (Variables|Default|GetToolWidget))))
  (if (> (Variables|/Game/MyMission/RightTool/W_CollectTools.W_CollectTools_C|GetMax%20Tools _asw_collect_tools) (Variables|/Game/MyMission/RightTool/W_CollectTools.W_CollectTools_C|GetCollected%20Tools _asw_collect_tools))
    (bind _output_get (Variables|/Game/MyMission/RightTool/W_CollectTools.W_CollectTools_C|SetCollected%20Tools _asw_collect_tools (+ (Variables|/Game/MyMission/RightTool/W_CollectTools.W_CollectTools_C|GetCollected%20Tools _asw_collect_tools) 1)))
    (Variables|Default|SetCollected%20Tools%20in%20collecter _output_get)
    (if (== (Variables|/Game/MyMission/RightTool/W_CollectTools.W_CollectTools_C|GetMax%20Tools _asw_collect_tools) (Variables|/Game/MyMission/RightTool/W_CollectTools.W_CollectTools_C|GetCollected%20Tools _asw_collect_tools))
      (Variables|Default|SetIs%20This%20Mission%20Complete? true)
      (Default|CallOnCompleted))))

(event Input|KeyboardEvents|Tab
  (params (Key :type Key%20Structure :default "None"))
  (:Pressed
    (if (not (Variables|Default|GetNot%20Completed?))
      (Variables|Default|SetNot%20Completed? true)
      (Variables|Default|SetIs%20This%20Mission%20Complete? true)
      (Rendering|SetVisibility (Variables|Default|GetCompleteWidget) true false)
      (bind _asw_collect_tools (Utilities|Casting|CastToW_CollectTools (UserInterface|GetUserWidgetObject (Variables|Default|GetToolWidget))))
      (Variables|/Game/MyMission/RightTool/W_CollectTools.W_CollectTools_C|SetCollected%20Tools _asw_collect_tools 3)
      (Variables|Default|SetCollected%20Tools%20in%20collecter 3)
      (Default|CallOnCompleted))))

(fn ConstructionScript)