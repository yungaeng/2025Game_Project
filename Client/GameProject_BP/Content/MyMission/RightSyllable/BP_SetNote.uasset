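; BP_SetNote is a set of eight solfège note trigger boxes, Do through high Do, for the RightSyllable mission.
; When BP_Adventurer overlaps a box, it plays that note's sound at the actor location and sends the note's index to BP_RandomNotePlayer actors found by class lookup.
; Box collision is disabled on BeginPlay and toggled through the EnableNoteCollision and DisableNoteCollision events.
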(event OnComponentBeginOverlap(DoBox)
  (params (OverlappedComponent :type Primitive%20Component%20Object%20Reference) (OtherActor :type Actor%20Object%20Reference) (OtherComp :type Primitive%20Component%20Object%20Reference) (OtherBodyIndex :type Integer) (bFromSweep :type Boolean) (SweepResult :type Hit%20Result%20Structure%20%28by%20ref%29))
  (Utilities|Casting|CastToBP_Adventurer OtherActor)
  (Audio|PlaySoundatLocation "/Game/MyMission/RightSyllable/Syllable/Do.Do" (Transformation|GetActorLocation) "0, 0, 0" 1.0 1.0 0.0 0 0 0 0)
  (bind _outactors (Actor|GetAllActorsOfClass "/Game/MyMission/RightSyllable/BP_RandomNotePlayer.BP_RandomNotePlayer_C"))
  (Default|AddNoteIndex _outactors))

(event OnComponentBeginOverlap(FaBox)
  (params (OverlappedComponent :type Primitive%20Component%20Object%20Reference) (OtherActor :type Actor%20Object%20Reference) (OtherComp :type Primitive%20Component%20Object%20Reference) (OtherBodyIndex :type Integer) (bFromSweep :type Boolean) (SweepResult :type Hit%20Result%20Structure%20%28by%20ref%29))
  (Utilities|Casting|CastToBP_Adventurer OtherActor)
  (Audio|PlaySoundatLocation "/Game/MyMission/RightSyllable/Syllable/Fa.Fa" (Transformation|GetActorLocation) "0, 0, 0" 1.0 1.0 0.0 0 0 0 0)
  (bind _outactors (Actor|GetAllActorsOfClass "/Game/MyMission/RightSyllable/BP_RandomNotePlayer.BP_RandomNotePlayer_C"))
  (Default|AddNoteIndex _outactors 3))

(event OnComponentBeginOverlap(MiBox)
  (params (OverlappedComponent :type Primitive%20Component%20Object%20Reference) (OtherActor :type Actor%20Object%20Reference) (OtherComp :type Primitive%20Component%20Object%20Reference) (OtherBodyIndex :type Integer) (bFromSweep :type Boolean) (SweepResult :type Hit%20Result%20Structure%20%28by%20ref%29))
  (Utilities|Casting|CastToBP_Adventurer OtherActor)
  (Audio|PlaySoundatLocation "/Game/MyMission/RightSyllable/Syllable/Mi.Mi" (Transformation|GetActorLocation) "0, 0, 0" 1.0 1.0 0.0 0 0 0 0)
  (bind _outactors (Actor|GetAllActorsOfClass "/Game/MyMission/RightSyllable/BP_RandomNotePlayer.BP_RandomNotePlayer_C"))
  (Default|AddNoteIndex _outactors 2))

(event OnComponentBeginOverlap(ReBox)
  (params (OverlappedComponent :type Primitive%20Component%20Object%20Reference) (OtherActor :type Actor%20Object%20Reference) (OtherComp :type Primitive%20Component%20Object%20Reference) (OtherBodyIndex :type Integer) (bFromSweep :type Boolean) (SweepResult :type Hit%20Result%20Structure%20%28by%20ref%29))
  (Utilities|Casting|CastToBP_Adventurer OtherActor)
  (Audio|PlaySoundatLocation "/Game/MyMission/RightSyllable/Syllable/Re.Re" (Transformation|GetActorLocation) "0, 0, 0" 1.0 1.0 0.0 0 0 0 0)
  (bind _outactors (Actor|GetAllActorsOfClass "/Game/MyMission/RightSyllable/BP_RandomNotePlayer.BP_RandomNotePlayer_C"))
  (Default|AddNoteIndex _outactors 1))

(event OnComponentBeginOverlap(SoBox)
  (params (OverlappedComponent :type Primitive%20Component%20Object%20Reference) (OtherActor :type Actor%20Object%20Reference) (OtherComp :type Primitive%20Component%20Object%20Reference) (OtherBodyIndex :type Integer) (bFromSweep :type Boolean) (SweepResult :type Hit%20Result%20Structure%20%28by%20ref%29))
  (Utilities|Casting|CastToBP_Adventurer OtherActor)
  (Audio|PlaySoundatLocation "/Game/MyMission/RightSyllable/Syllable/So.So" (Transformation|GetActorLocation) "0, 0, 0" 1.0 1.0 0.0 0 0 0 0)
  (bind _outactors (Actor|GetAllActorsOfClass "/Game/MyMission/RightSyllable/BP_RandomNotePlayer.BP_RandomNotePlayer_C"))
  (Default|AddNoteIndex _outactors 4))

(event OnComponentBeginOverlap(HDoBox)
  (params (OverlappedComponent :type Primitive%20Component%20Object%20Reference) (OtherActor :type Actor%20Object%20Reference) (OtherComp :type Primitive%20Component%20Object%20Reference) (OtherBodyIndex :type Integer) (bFromSweep :type Boolean) (SweepResult :type Hit%20Result%20Structure%20%28by%20ref%29))
  (Utilities|Casting|CastToBP_Adventurer OtherActor)
  (Audio|PlaySoundatLocation "/Game/MyMission/RightSyllable/Syllable/HDo.HDo" (Transformation|GetActorLocation) "0, 0, 0" 1.0 1.0 0.0 0 0 0 0)
  (bind _outactors (Actor|GetAllActorsOfClass "/Game/MyMission/RightSyllable/BP_RandomNotePlayer.BP_RandomNotePlayer_C"))
  (Default|AddNoteIndex _outactors 7))

(event OnComponentBeginOverlap(LaBox)
  (params (OverlappedComponent :type Primitive%20Component%20Object%20Reference) (OtherActor :type Actor%20Object%20Reference) (OtherComp :type Primitive%20Component%20Object%20Reference) (OtherBodyIndex :type Integer) (bFromSweep :type Boolean) (SweepResult :type Hit%20Result%20Structure%20%28by%20ref%29))
  (Utilities|Casting|CastToBP_Adventurer OtherActor)
  (Audio|PlaySoundatLocation "/Game/MyMission/RightSyllable/Syllable/La.La" (Transformation|GetActorLocation) "0, 0, 0" 1.0 1.0 0.0 0 0 0 0)
  (bind _outactors (Actor|GetAllActorsOfClass "/Game/MyMission/RightSyllable/BP_RandomNotePlayer.BP_RandomNotePlayer_C"))
  (Default|AddNoteIndex _outactors 5))

(event OnComponentBeginOverlap(TiBox)
  (params (OverlappedComponent :type Primitive%20Component%20Object%20Reference) (OtherActor :type Actor%20Object%20Reference) (OtherComp :type Primitive%20Component%20Object%20Reference) (OtherBodyIndex :type Integer) (bFromSweep :type Boolean) (SweepResult :type Hit%20Result%20Structure%20%28by%20ref%29))
  (Utilities|Casting|CastToBP_Adventurer OtherActor)
  (Audio|PlaySoundatLocation "/Game/MyMission/RightSyllable/Syllable/Ti.Ti" (Transformation|GetActorLocation) "0, 0, 0" 1.0 1.0 0.0 0 0 0 0)
  (bind _outactors (Actor|GetAllActorsOfClass "/Game/MyMission/RightSyllable/BP_RandomNotePlayer.BP_RandomNotePlayer_C"))
  (Default|AddNoteIndex _outactors 6))

(event Custom|EnableNoteCollision
  (Collision|SetCollisionEnabled (Variables|Default|GetDoBox) "QueryOnly"))

(event Custom|Disable%20Note%20Collision
  (Collision|SetCollisionEnabled (Variables|Default|GetDoBox) "NoCollision"))

(event EventBeginPlay
  (CallFunction|DisableNoteCollision))

(fn ConstructionScript)