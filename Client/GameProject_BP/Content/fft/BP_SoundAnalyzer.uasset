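; BP_SoundAnalyzer is an actor that detects the pitch of captured audio and prints the note name on screen.
; Entering its Sphere overlap activates the AudioCapture component, and leaving it deactivates the capture.
; On BeginPlay it binds GetTone to the PitchDetector's pitch-detected event, which prints each detected note.
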(event OnComponentBeginOverlap(Sphere)
  (params (OverlappedComponent :type Primitive%20Component%20Object%20Reference) (OtherActor :type Actor%20Object%20Reference) (OtherComp :type Primitive%20Component%20Object%20Reference) (OtherBodyIndex :type Integer) (bFromSweep :type Boolean) (SweepResult :type Hit%20Result%20Structure%20%28by%20ref%29))
  (Components|Activation|Activate (Variables|Default|GetAudioCapture) false))

(event OnComponentEndOverlap(Sphere)
  (params (OverlappedComponent :type Primitive%20Component%20Object%20Reference) (OtherActor :type Actor%20Object%20Reference) (OtherComp :type Primitive%20Component%20Object%20Reference) (OtherBodyIndex :type Integer))
  (Components|Activation|Deactivate (Variables|Default|GetAudioCapture)))

(event Custom|GetTone
  (params (PitchInfo :type Pitch%20Info%20Structure%20%28by%20ref%29))
  (Development|PrintString (.NoteName (Utilities|Struct|BreakPitchInfo PitchInfo))))

(event EventBeginPlay
  (EventDispatchers|BindEventtoOnPitchDetected (Variables|Default|GetPitchDetector) (delegate Custom|GetTone)))

(fn ConstructionScript)