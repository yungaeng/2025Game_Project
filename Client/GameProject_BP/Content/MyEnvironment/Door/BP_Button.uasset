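; BP_Button is a pressable button that broadcasts an OpenDoor event, triggered by the player or a weapon.
; BP_Adventurer overlapping Box enables input and opens a gate for the Interact action; leaving reverses both.
; Interact, or a component tagged ImposterWeapon entering Box1, plays a Timeline that offsets the mesh along relative Y.
; OpenDoor fires on every Timeline update, and the gate reopens when it finishes.
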(event OnComponentBeginOverlap(Box1)
  (params (OverlappedComponent :type Primitive%20Component%20Object%20Reference) (OtherActor :type Actor%20Object%20Reference) (OtherComp :type Primitive%20Component%20Object%20Reference) (OtherBodyIndex :type Integer) (bFromSweep :type Boolean) (SweepResult :type Hit%20Result%20Structure%20%28by%20ref%29))
  (bind _button_transform (Variables|Default|GetButton%20Transform))
  (if (Components|ComponentHasTag OtherComp "ImposterWeapon")
    (bind _button_track (Timeline|Timeline PlayFromStart)
      (:Update
        (Transformation|SetRelativeLocation (Variables|Debug|GetStaticMeshComponent) (Math|Vector|MakeVector (.x (.location _button_transform)) (+ _button_track (.y (.location _button_transform))) (.z (.location _button_transform))) false false)
        (Default|CallOpenDoor))
      (:Finished
        (Utilities|FlowControl|Gate true) ; enters at Open
      ))))

(event OnComponentBeginOverlap(Box)
  (params (OverlappedComponent :type Primitive%20Component%20Object%20Reference) (OtherActor :type Actor%20Object%20Reference) (OtherComp :type Primitive%20Component%20Object%20Reference) (OtherBodyIndex :type Integer) (bFromSweep :type Boolean) (SweepResult :type Hit%20Result%20Structure%20%28by%20ref%29))
  (bind _button_transform (Variables|Default|GetButton%20Transform))
  (Utilities|Casting|CastToBP_Adventurer OtherActor)
  (Input|EnableInput (Game|GetPlayerController 0))
  (Utilities|FlowControl|Gate true) ; enters at Open
)

(event OnComponentEndOverlap(Box)
  (params (OverlappedComponent :type Primitive%20Component%20Object%20Reference) (OtherActor :type Actor%20Object%20Reference) (OtherComp :type Primitive%20Component%20Object%20Reference) (OtherBodyIndex :type Integer))
  (bind _button_transform (Variables|Default|GetButton%20Transform))
  (Utilities|Casting|CastToBP_Adventurer OtherActor)
  (Input|DisableInput (Game|GetPlayerController 0))
  (Utilities|FlowControl|Gate true) ; enters at Close
)

(event EventBeginPlay
  (Input|EnableInput (Game|GetPlayerController 0))
  (Variables|Default|SetButton%20Transform (Transformation|GetRelativeTransform (Variables|Debug|GetStaticMeshComponent))))

(event Input|ActionEvents|InputActionInteract
  (params (Key :type Key%20Structure :default "None"))
  (bind _button_transform (Variables|Default|GetButton%20Transform))
  (:Pressed
    (Utilities|FlowControl|Gate true :!label _label
      (:Exit
        (bind _button_track (Timeline|Timeline PlayFromStart)
          (:Update
            (Transformation|SetRelativeLocation (Variables|Debug|GetStaticMeshComponent) (Math|Vector|MakeVector (.x (.location _button_transform)) (+ _button_track (.y (.location _button_transform))) (.z (.location _button_transform))) false false)
            (Default|CallOpenDoor))
          (:Finished
            (goto _label Open)))))))

(fn ConstructionScript)