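; BP_Door2 is a sliding door that opens from either of two linked button references and closes itself after a short delay.
; On BeginPlay it caches the mesh's relative transform and binds both buttons to its Button event, which ignores presses until the door is closed again.
; A Timeline offsets the mesh along its right vector.
; A FlipFlop on Finished alternates between delayed reverse playback and re-arming the door.
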(event Custom|Button
  (if (Variables|Default|GetIs%20Door%20Close?)
    (Variables|Default|SetIs%20Door%20Close? false)
    (bind _door_track (Timeline|Timeline Play)
      (:Update
        (Transformation|SetRelativeLocation (Variables|Debug|GetStaticMeshComponent) (+ (* _door_track (Math|Vector|GetRightVector (Variables|Debug|GetStaticMeshComponent))) (.location (Variables|Default|GetDoor%20Transform))) false false))
      (:Finished
        (Utilities|FlowControl|FlipFlop
          (:A
            (Utilities|FlowControl|Delay 5.0)
            (Timeline|Timeline Reverse))
          (:B
            (Variables|Default|SetIs%20Door%20Close? true)))))))

(event EventBeginPlay
  (Variables|Default|SetDoor%20Transform (Transformation|GetRelativeTransform (Variables|Debug|GetStaticMeshComponent)))
  (EventDispatchers|BindEventtoOpenDoor (Variables|Default|GetButton%20Click_1) (delegate Custom|Button)))

(fn ConstructionScript)