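; Interactable microphone pitch-analyzer station for a mission, usable while BP_Adventurer is inside its trigger sphere.
; Interact toggles the W_NoteDisplay widget, locking move and look input and running mic capture only while the mission is incomplete.
; AudioCapture feeds an analyzer submix, and PitchDetector callbacks push note name and volume to the widget.
; Cleared stops capture, marks the mission complete and calls SoundAnalyzerClear; Tab calls the widget's Clear.
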(event OnComponentBeginOverlap(Sphere)
  (params (OverlappedComponent :type Primitive%20Component%20Object%20Reference) (OtherActor :type Actor%20Object%20Reference) (OtherComp :type Primitive%20Component%20Object%20Reference) (OtherBodyIndex :type Integer) (bFromSweep :type Boolean) (SweepResult :type Hit%20Result%20Structure%20%28by%20ref%29))
  (Utilities|Casting|CastToBP_Adventurer OtherActor)
  (Input|EnableInput (Game|GetPlayerController 0)))

(event OnComponentEndOverlap(Sphere)
  (params (OverlappedComponent :type Primitive%20Component%20Object%20Reference) (OtherActor :type Actor%20Object%20Reference) (OtherComp :type Primitive%20Component%20Object%20Reference) (OtherBodyIndex :type Integer))
  (Input|DisableInput (Game|GetPlayerController 0)))

(event Custom|GetTone
  (params (PitchInfo :type Pitch%20Info%20Structure%20%28by%20ref%29))
  (bind (_frequency _notename _confidence _volume) (Utilities|Struct|BreakPitchInfo PitchInfo))
  (bind _output_get (Variables|Default|SetNotename _notename))
  (Default|UpdateMicNote (Variables|Default|Get%20W%20Note%20Display) _output_get _volume)
  (if (> _volume 4e+01)
    (Variables|Default|SetLoud true)
    (else
      (Variables|Default|SetLoud false))))

(event Custom|Cleared
  (bind _audiocapture (Variables|Default|GetAudioCapture))
  (Components|Activation|Deactivate (Variables|Default|GetPitchDetector))
  (Components|Activation|Deactivate _audiocapture)
  (Audio|Components|Audio|Stop _audiocapture)
  (Variables|Default|SetIs%20This%20Mission%20Complete? true)
  (Default|CallSoundAnalyzerClear))

(event EventBeginPlay
  (Audio|Components|Audio|SetSubmixSend (Variables|Default|GetAudioCapture) "/Game/MyFFT/SM_Analyzer.SM_Analyzer" 1.0 :!class /Script/AudioMixer.SynthComponent)
  (bind _returnvalue (UserInterface|CreateWidget "/Game/MyFFT/W_NoteDisplay.W_NoteDisplay_C" 0 self))
  (Variables|Default|Set%20W%20Note%20Display _returnvalue)
  (EventDispatchers|BindEventtoOnPitchDetected (Variables|Default|GetPitchDetector) (delegate Custom|GetTone)))

(event EventEndPlay
  (params (EndPlayReason :type EEndPlayReason%20Enum :default "Destroyed"))
  (Utilities|IsValid (Variables|Default|GetPitchDetector)
    (:Is%20Valid
      (Class|PitchDetectorComponent|CleanupSubmix (Variables|Default|GetPitchDetector)))))

(event Input|ActionEvents|InputActionInteract
  (params (Key :type Key%20Structure :default "None"))
  (bind _returnvalue (Game|GetPlayerController 0))
  (bind _returnvalue_2 (Game|GetPlayerController 0))
  (bind _returnvalue_3 (Game|GetPlayerController 0))
  (bind _audiocapture (Variables|Default|GetAudioCapture))
  (bind _audiocapture_2 (Variables|Default|GetAudioCapture))
  (bind _audiocapture_3 (Variables|Default|GetAudioCapture))
  (:Pressed
    (if (Variables|Default|GetIsWidgetOpen?)
      (Widget|RemovefromParent (Variables|Default|Get%20W%20Note%20Display))
      (Variables|Default|SetIsWidgetOpen? false)
      (Input|SetInputModeGameOnly _returnvalue_2 true)
      (Input|SetIgnoreMoveInput _returnvalue_2 false)
      (Input|SetIgnoreLookInput _returnvalue_2 false)
      (Components|Activation|Deactivate (Variables|Default|GetPitchDetector))
      (Components|Activation|Deactivate _audiocapture)
      (Audio|Components|Audio|Stop _audiocapture)
      (else
        (UserInterface|Viewport|AddtoViewport (Variables|Default|Get%20W%20Note%20Display) 0)
        (Audio|PlaySound2D "/Game/MyFFT/pop.pop" 1.0 1.0 0.0 0 0)
        (if (Variables|Default|GetIs%20This%20Mission%20Complete?)
          (Input|SetIgnoreMoveInput _returnvalue_3 true)
          (Input|SetIgnoreLookInput _returnvalue_3 true)
          (Input|SetInputModeGameandUI _returnvalue_3 (Variables|Default|Get%20W%20Note%20Display) "LockAlways" true false)
          (Components|Activation|Deactivate (Variables|Default|GetPitchDetector))
          (Components|Activation|Deactivate _audiocapture_2)
          (Audio|Components|Audio|Stop _audiocapture_2)
          (Variables|Default|SetIsWidgetOpen? true)
          (else
            (bind _asw_note_display (Utilities|Casting|CastToW_NoteDisplay (Variables|Default|Get%20W%20Note%20Display)))
            (Default|Reset! _asw_note_display)
            (Variables|Default|SetIsWidgetOpen? true)
            (Input|SetIgnoreMoveInput _returnvalue true)
            (Input|SetIgnoreLookInput _returnvalue true)
            (Input|SetInputModeGameandUI _returnvalue (Variables|Default|Get%20W%20Note%20Display) "LockAlways" true false)
            (Components|Activation|Activate (Variables|Default|GetPitchDetector) false)
            (Components|Activation|Activate _audiocapture_3 false)
            (CameraShake|Start _audiocapture_3)))))))

(event Input|KeyboardEvents|Tab
  (params (Key :type Key%20Structure :default "None"))
  (:Pressed
    (bind _asw_note_display (Utilities|Casting|CastToW_NoteDisplay (Variables|Default|Get%20W%20Note%20Display)))
    (Default|Clear! _asw_note_display)))

(fn ConstructionScript)

(fn AddEcho)