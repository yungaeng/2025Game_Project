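; BP_tool is an interactable tool actor that BP_Adventurer collects by pressing Interact while in range.
; Its Sphere's overlap events store or clear the current adventurer and enable or disable the actor's input for player controller 0.
; The Interact press calls ToolCollect on the stored adventurer, leaving all collection logic to that character, as the tool does not hide or destroy itself.
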(event OnComponentBeginOverlap(Sphere)
  (params (OverlappedComponent :type Primitive%20Component%20Object%20Reference) (OtherActor :type Actor%20Object%20Reference) (OtherComp :type Primitive%20Component%20Object%20Reference) (OtherBodyIndex :type Integer) (bFromSweep :type Boolean) (SweepResult :type Hit%20Result%20Structure%20%28by%20ref%29))
  (Utilities|Casting|CastToBP_Adventurer OtherActor)
  (Variables|Default|SetCurrent%20Overlapping%20Actor OtherActor)
  (Input|EnableInput (Game|GetPlayerController 0)))

(event OnComponentEndOverlap(Sphere)
  (params (OverlappedComponent :type Primitive%20Component%20Object%20Reference) (OtherActor :type Actor%20Object%20Reference) (OtherComp :type Primitive%20Component%20Object%20Reference) (OtherBodyIndex :type Integer))
  (Utilities|Casting|CastToBP_Adventurer OtherActor)
  (Variables|Default|SetCurrent%20Overlapping%20Actor 0)
  (Input|DisableInput (Game|GetPlayerController 0)))

(event EventBeginPlay)

(event Collision|EventActorBeginOverlap
  (params (OtherActor :type Actor%20Object%20Reference)))

(event EventTick
  (params (DeltaSeconds :type Float%20%28single-precision%29)))

(event Input|ActionEvents|InputActionInteract
  (params (Key :type Key%20Structure :default "None"))
  (:Pressed
    (bind _asbp_adventurer (Utilities|Casting|CastToBP_Adventurer (Variables|Default|GetCurrent%20Overlapping%20Actor)))
    (Default|ToolCollect _asbp_adventurer)))

(fn ConstructionScript)