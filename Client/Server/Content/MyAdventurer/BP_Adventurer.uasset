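; Player character for the Adventurer side against BP_Imposter, with minimap, target indicators, tool carrying into collectors, and hit-based death and respawn that reduces the world timer.
; Sprinting drains stamina through delayed recursive events, and footstep notifies spawn echo actors given the Imposter's camera.
; On remote clients the Imposter's mesh and weapon are hidden until battery-timed thermal vision swaps camera post-process, revealing them and toggling heater temperature vision.
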(event OnComponentBeginOverlap(CapsuleComponent)
  (params (OverlappedComponent :type Primitive%20Component%20Object%20Reference) (OtherActor :type Actor%20Object%20Reference) (OtherComp :type Primitive%20Component%20Object%20Reference) (OtherBodyIndex :type Integer) (bFromSweep :type Boolean) (SweepResult :type Hit%20Result%20Structure%20%28by%20ref%29))
  (if (not (Variables|Default|GetIs%20Holding?))
    (bind _asbp_tool (Utilities|Casting|CastToBP_tool OtherActor))
    (Variables|Default|SetOverlapping%20Item _asbp_tool)))

(event OnComponentEndOverlap(CapsuleComponent)
  (params (OverlappedComponent :type Primitive%20Component%20Object%20Reference) (OtherActor :type Actor%20Object%20Reference) (OtherComp :type Primitive%20Component%20Object%20Reference) (OtherBodyIndex :type Integer))
  (bind _asbp_tool (Utilities|Casting|CastToBP_tool OtherActor))
  (Variables|Default|SetOverlapping%20Item _asbp_tool))

(event Custom|Decrease%20Timer
  (if (> (Variables|Default|GetBattery%20Time) 0.0)
    (Variables|Default|SetBattery%20Time (- (Variables|Default|GetBattery%20Time) 1.0))
    (else
      (Widget|SetVisibility (Variables|Default|GetThermal%20Vision%20Widget) "Hidden")
      (Variables|/Script/Engine.CameraComponent|SetPostProcessSettings (Variables|Default|GetCamera) "")
      (Utilities|Time|SetTimerbyFunctionName 0 "Decrease Timer" 0.0)
      (Variables|Default|SetIs%20Thermal%20Vision%20Hidden? true)
      (Rendering|SetVisibility (Variables|Default|GetImposter%20Weapon) false false)
      (CallFunction|MakeHeaterThermalVision false))))

(event Custom|TakeDamage
  (Audio|PlaySound2D "/Game/MyImposter/hard-slap.hard-slap" 0.2 1.0 0.0 0 0)
  (Variables|Default|SetHitCount (- (Variables|Default|GetHitCount) 1))
  (if (== (Variables|Default|GetHitCount) 0)
    (bind _foundwidgets (Widget|GetAllWidgetsOfClass "/Game/MyEnvironment/W_WorldTimer.W_WorldTimer_C" true))
    (Default|ReduceTimer _foundwidgets)
    (Animation|Montage|PlayMontage (Variables|Character|GetMesh) "/Game/MyAdventurer/AdventurerAnimation/dead_Montage.dead_Montage"
      (:then
        (Input|DisableInput 0)
        (Collision|SetCollisionEnabled (Variables|Collision|GetCapsuleComponent) "NoCollision")
        (Input|SetIgnoreLookInput (Game|GetPlayerController 0) true)
        (Utilities|FlowControl|Delay 3.0)
        (Animation|StopAnimMontage "/Game/MyAdventurer/AdventurerAnimation/dead_Montage.dead_Montage")
        (bind _outactors (Actor|GetAllActorsOfClass "/Game/MyAdventurer/BP_RespawnPos.BP_RespawnPos_C"))
        (Transformation|SetActorLocation (Transformation|GetActorLocation (Utilities|Array|Get(acopy) _outactors)) false false)
        (Collision|SetCollisionEnabled (Variables|Collision|GetCapsuleComponent) "QueryAndPhysics")
        (Input|EnableInput 0)
        (Input|SetIgnoreLookInput (Game|GetPlayerController 0) false)
        (Variables|Default|SetHitCount 3)
        (Variables|Default|SetTotal%20Hit (+ (Variables|Default|GetTotal%20Hit) 1))))))

(event Custom|Tool%20Collect
  (bind _overlapping_item (Variables|Default|GetOverlapping%20Item))
  (Utilities|IsValid (Variables|Default|GetOverlapping%20Item)
    (:Is%20Valid
      (if (Variables|Default|GetIs%20Holding?)
        (bind (_outhit _returnvalue) (Collision|LineTraceByChannel (Transformation|GetActorLocation) (- (Transformation|GetActorLocation) (Math|Vector|MakeVector 0.0 0.0 5e+02)) "TraceTypeQuery1" false 0 "None"))
        (if _returnvalue
          (Utilities|IsValid (Variables|Default|GetOverlapping%20Item)
            (:Is%20Valid
              (Transformation|DetachFromActor _overlapping_item "KeepWorld" "KeepWorld" "KeepWorld")
              (Transformation|SetActorTransform _overlapping_item (Math|Transform|MakeTransform (+ (.Location (Collision|BreakHitResult _outhit)) "0.000000,0.000000,13.000000") "0, 0, 0" "1.500000,1.500000,1.500000"))
              (Variables|Default|SetIs%20Holding? false)
              (for _array_element (Collision|GetOverlappingActors "/Game/MyMission/RightTool/BP_ToolCollecter.BP_ToolCollecter_C" :!class /Script/Engine.Actor)
                (bind _asbp_tool_collecter (Utilities|Casting|CastToBP_ToolCollecter _array_element))
                (if (< (Variables|/Game/MyMission/RightTool/BP_ToolCollecter.BP_ToolCollecter_C|GetCollected%20Tools%20in%20collecter _asbp_tool_collecter) (Variables|/Game/MyMission/RightTool/BP_ToolCollecter.BP_ToolCollecter_C|GetMax%20Tools%20in%20collecter _asbp_tool_collecter))
                  (Default|UpdateCollecterCount _asbp_tool_collecter)
                  (Actor|DestroyActor (Variables|Default|GetOverlapping%20Item)))))))
        (else
          (Transformation|AttachComponentToComponent (Variables|Default|GetOverlapping%20Item) (Variables|Character|GetMesh) "ItemSocket" "SnapToTarget" "SnapToTarget" "SnapToTarget" true)
          (Variables|Default|SetIs%20Holding? true))))))

(event Custom|Fixed%20Temperature
  (Variables|Default|GetTarget%20Heater
    (:then)
    (:else)))

(event Custom|Battery%20Collect
  (Variables|Default|SetBattery%20Time (+ (Variables|Default|GetBattery%20Time) (Variables|Default|GetMax%20Battery%20Time)))
  (if (>= (Variables|Default|GetBattery%20Time) (Variables|Default|GetMax%20Battery%20Time))
    (Variables|Default|SetBattery%20Time (+ (Variables|Default|GetMax%20Battery%20Time) 1.0))))

(event Custom|Decrease%20Stamina
  (Widget|SetVisibility (Variables|Default|GetStamina%20Widget) "Visible")
  (bind _output_get (Variables|Default|SetStamina (Math|Integer|Clamp(Integer) (- (Variables|Default|GetStamina) 1) 0 (Variables|Default|GetMax%20Stamina))))
  (if (== _output_get 0)
    (CallFunction|StopRunning)
    (elif (Variables|Default|GetIs%20Running?)
      (Utilities|FlowControl|Delay 0.1)
      (CallFunction|DecreaseStamina))))

(event Custom|Increase%20Stamina
  (bind _output_get (Variables|Default|SetStamina (Math|Integer|Clamp(Integer) (+ (Variables|Default|GetStamina) 1) 0 (Variables|Default|GetMax%20Stamina))))
  (if (== _output_get (Variables|Default|GetMax%20Stamina))
    (Widget|SetVisibility (Variables|Default|GetStamina%20Widget) "Hidden")
    (elif (not (Variables|Default|GetIs%20Running?))
      (Utilities|FlowControl|Delay 0.1)
      (CallFunction|IncreaseStamina))))

(event Custom|CE_RunFootNotify
  (bind _outactors (Actor|GetAllActorsOfClass "/Game/MyImposter/BP_Imposter.BP_Imposter_C"))
  (bind _asbp_imposter (Utilities|Casting|CastToBP_Imposter (Utilities|Array|Get(acopy) _outactors)))
  (Game|SpawnActorfromClass "/Game/Echolation/A_EchoGenerate2.A_EchoGenerate2_C" (Math|Transform|MakeTransform (Transformation|GetActorLocation) "0, 0, 0" "1.000000,1.000000,1.000000") "Undefined" "MultiplyWithRoot" 0 "(R=1.000000,G=1.000000,B=1.000000,A=1.000000)" 7e+02 0.0 (Variables|/Game/MyImposter/BP_Imposter.BP_Imposter_C|GetCameraImposter _asbp_imposter) 0))

(event Custom|CE_FootNotify
  (bind _outactors (Actor|GetAllActorsOfClass "/Game/MyImposter/BP_Imposter.BP_Imposter_C"))
  (bind _asbp_imposter (Utilities|Casting|CastToBP_Imposter (Utilities|Array|Get(acopy) _outactors)))
  (Game|SpawnActorfromClass "/Game/MyEcholation/A_EchoGenerate.A_EchoGenerate_C" (Math|Transform|MakeTransform (Transformation|GetActorLocation) "0, 0, 0" "1.000000,1.000000,1.000000") "Undefined" "MultiplyWithRoot" 0 "(R=1.000000,G=1.000000,B=1.000000,A=1.000000)" 5e+02 0.0 (Variables|/Game/MyImposter/BP_Imposter.BP_Imposter_C|GetCameraImposter _asbp_imposter) 0))

(event Custom|SoundAnalyzer_Echo)

(event Input|EnhancedActionEvents|EnhancedInputActionIA_Jump_I
  (params (ActionValue :type Boolean) (ElapsedSeconds :type Float%20%28double-precision%29) (TriggeredSeconds :type Float%20%28double-precision%29) (InputAction :type Input%20Action%20Object%20Reference :default "/Game/MyImposter/IA_Jump_I.IA_Jump_I"))
  (:Started
    (Character|Jump)))

(event EventBeginPlay
  (bind _returnvalue (Pawn|GetController))
  ;[1 1 1] 한 프레임 뒤로 미는 노드 없으면 크래시 남
  (Utilities|FlowControl|DelayUntilNextTick)
  ;[1 1 1] 시작할때 스테미나 등록, 시작할땐 안보이게
  (bind _returnvalue_2 (UserInterface|CreateWidget "/Game/MyAdventurer/W_Stamina.W_Stamina_C"))
  (bind _output_get (Variables|Default|SetStamina%20Widget _returnvalue_2))
  (UserInterface|Viewport|AddtoViewport _output_get 0)
  (Widget|SetVisibility (Variables|Default|GetStamina%20Widget) "Hidden")
  (CallFunction|IncreaseStamina)
  (Utilities|IsValid _returnvalue
    (:Is%20Valid
      (if (Pawn|IsLocalController _returnvalue)
        (bind _returnvalue_3 (UserInterface|CreateWidget "/Game/Minimap/W_Minimap.W_Minimap_C"))
        (bind _output_get_2 (Variables|Default|SetMinimap%20Widget _returnvalue_3))
        (UserInterface|Viewport|AddtoViewport _output_get_2 0)
        (Utilities|FlowControl|Delay 0.2)
        (bind _outactors (Actor|GetAllActorsOfClass "BP_Adventurer_C"))
        (for _array_element _outactors
          (if (!= _array_element self)
            (Utilities|Array|Add (Variables|Default|GetIndicater%20Target%20Actors) _array_element)
            (bind _outactors_2 (Actor|GetAllActorsOfClass "/Game/MyImposter/BP_Imposter.BP_Imposter_C"))
            (for _array_element_2 _outactors_2
              (Utilities|Array|Add (Variables|Default|GetIndicater%20Target%20Actors) _array_element_2)
              (for _array_element_3 (Variables|Default|GetIndicater%20Target%20Actors)
                (bind _asmy_player_controller (Utilities|Casting|CastToMyPlayerController (Pawn|GetController)))
                (bind _returnvalue_4 (UserInterface|CreateWidget "/Game/MyAdventurer/W_Indicater.W_Indicater_C" _asmy_player_controller _array_element_3))
                (UserInterface|Viewport|AddtoViewport _returnvalue_4 0)
                (Networking|SwitchHasAuthority
                  (:Remote
                    (bind _outactors_3 (Actor|GetAllActorsOfClass "/Game/MyImposter/BP_Imposter.BP_Imposter_C"))
                    (Utilities|IsValid (Utilities|Array|Get(acopy) _outactors_3)
                      (:Is%20Valid
                        (bind _output_get_3 (Variables|Default|SetBP_Imposter_Ref (Utilities|Array|Get(acopy) _outactors_3)))
                        (bind _output_get_4 (Variables|Default|SetImposter%20Mesh (Variables|/Script/Engine.Character|GetMesh _output_get_3)))
                        (bind _output_get_5 (Variables|Default|SetImposter%20Weapon (Variables|/Game/MyImposter/BP_Imposter.BP_Imposter_C|GetImposterWeapon _output_get_3)))
                        (Rendering|SetVisibility _output_get_5 false false)))))))))))))

(event EventTick
  (params (DeltaSeconds :type Float%20%28single-precision%29))
  (bind _returnvalue (Game|GetPlayerCharacter 0))
  (bind _returnvalue_2 (Transformation|GetActorRotation _returnvalue))
  (bind _yaw (Math|Rotator|BreakRotator _returnvalue_2))
  ;[1 1 1] 캐릭터의 속도를 저장한다.
  (Variables|Default|SetGround%20Speed (Math|Vector|VectorLengthXY (Variables|/Script/Engine.MovementComponent|GetVelocity (Variables|Character|GetCharacterMovement))))
  (Rendering|Material|SetVectorParameterValue "/Game/Minimap/MP_Minimap.MP_Minimap" "Player Location" (Math|Conversions|ToLinearColor(Vector) (Transformation|GetActorLocation _returnvalue)) :!class /Script/Engine.KismetMaterialLibrary)
  (Rendering|Material|SetScalarParameterValue "/Game/Minimap/MP_Minimap.MP_Minimap" "Player Yaw" (/ (Math|Float|SelectFloat (- _yaw 3.6e+02) _yaw (< _yaw 0.0)) 3.6e+02) :!class /Script/Engine.KismetMaterialLibrary))

(event Input|KeyboardEvents|LeftShift
  (params (Key :type Key%20Structure :default "None"))
  (:Pressed
    (CallFunction|StartRunning))
  (:Released
    (CallFunction|StopRunning)))

(event Input|KeyboardEvents|V
  (params (Key :type Key%20Structure :default "None"))
  (bind _camera (Variables|Default|GetCamera))
  (bind _imposter_weapon (Variables|Default|GetImposter%20Weapon))
  (:Pressed
    (if (Variables|Default|GetIs%20Thermal%20Vision%20create?)
      _
      (else
        (bind _returnvalue (UserInterface|CreateWidget "/Game/MyAdventurer/W_ThermalVisonTimer.W_ThermalVisonTimer_C" (Game|GetPlayerController 0)))
        (bind _output_get (Variables|Default|SetThermal%20Vision%20Widget _returnvalue))
        (UserInterface|Viewport|AddtoViewport _output_get 0)
        (Variables|Default|SetIs%20Thermal%20Vision%20create? true)))
    (Networking|SwitchHasAuthority
      (:Remote
        (if (Variables|Default|GetIs%20Thermal%20Vision%20Hidden?)
          (if (> (Variables|Default|GetBattery%20Time) 0.0)
            (Variables|/Script/Engine.CameraComponent|SetPostProcessSettings _camera (Variables|Default|GetThermal%20Vison))
            (Widget|SetVisibility (Variables|Default|GetThermal%20Vision%20Widget) "Visible")
            (Utilities|Time|SetTimerbyFunctionName 0 "Decrease Timer" 1.0 true)
            (Variables|Default|SetIs%20Thermal%20Vision%20Hidden? false)
            (Rendering|SetVisibility _imposter_weapon true false)
            (CallFunction|MakeHeaterThermalVision true))
          (else
            (Variables|/Script/Engine.CameraComponent|SetPostProcessSettings _camera "")
            (Widget|SetVisibility (Variables|Default|GetThermal%20Vision%20Widget) "Collapsed")
            (Utilities|Time|SetTimerbyFunctionName 0 "Decrease Timer" 0.0)
            (Variables|Default|SetIs%20Thermal%20Vision%20Hidden? true)
            (Rendering|SetVisibility _imposter_weapon false false)
            (CallFunction|MakeHeaterThermalVision false)))))))

(fn ConstructionScript)

(fn MakeHeaterThermalVision
  (params (On :type Boolean))
  (bind _outactors (Actor|GetAllActorsOfClass "/Game/MyMission/FixTemperature/BP_FixTemperature.BP_FixTemperature_C"))
  (for _array_element _outactors
    (Default|ToggleTempVision _array_element On)))

(fn StartRunning
  (Variables|/Script/Engine.CharacterMovementComponent|SetMaxWalkSpeed (Variables|Character|GetCharacterMovement) 6e+02)
  (Variables|Default|SetIs%20Running? true)
  (CallFunction|DecreaseStamina))

(fn StopRunning
  (Variables|/Script/Engine.CharacterMovementComponent|SetMaxWalkSpeed (Variables|Character|GetCharacterMovement) 3e+02)
  (Variables|Default|SetIs%20Running? false)
  (CallFunction|IncreaseStamina))

(fn CleanUpBeforeTravel)